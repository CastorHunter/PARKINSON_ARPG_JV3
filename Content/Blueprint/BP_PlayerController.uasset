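; Player controller for a click-to-move spellcaster, handling movement, spell casting, trader buying and the player HUD.
; Mouse wheel cycles a growable spell library, and A freezes movement while the active spell's animation plays, launching it through timed delays.
; Events implement fireball, earthquake and a timeline-driven rotating shield.
; A looping delay regenerates health and mana up to maximums captured from starting values, updating the UI.
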(event Custom|StopBuying
  (Default|StopBuying (CallFunction|GetPlayer))
  (Variables|Default|SetPlayerIsFrozen false))

(event Custom|SetPlayerUI
  (bind _player (CallFunction|GetPlayer))
  (bind _mana (Variables|/Game/Blueprint/BP_Character.BP_Character_C|GetMana _player))
  (bind _health (Variables|/Game/Blueprint/BP_Character.BP_Character_C|GetHealth _player))
  (bind _returnvalue (Math|Conversions|ToFloat(Integer) _mana))
  (bind _returnvalue_2 (Math|Conversions|ToFloat(Integer) _health))
  (Viewport|RemoveAllWidgets)
  (bind _returnvalue_3 (UserInterface|CreateWidget "/Game/Blueprint/WBP_PlayerUI.WBP_PlayerUI_C" self))
  (UserInterface|Viewport|AddtoPlayerScreen _returnvalue_3)
  (Variables|Default|SetPlayerUI _returnvalue_3)
  (Utilities|FlowControl|Delay 0.05)
  (Default|SetManaMax (Variables|Default|GetPlayerUI) _returnvalue)
  (Variables|Default|SetManaMax _returnvalue)
  (Default|UpdateMana (Variables|Default|GetPlayerUI) _returnvalue)
  (Default|SetHealthMax (Variables|Default|GetPlayerUI) _returnvalue_2)
  (Variables|Default|SetHealthMax _returnvalue_2)
  (Default|UpdateHealth (Variables|Default|GetPlayerUI) _returnvalue_2)
  (Default|UpdateActiveSpell (Variables|Default|GetPlayerUI) (Variables|/Game/DataAsset/BP_DA_Spell.BP_DA_Spell_C|GetName (Variables|Default|GetActiveSpell)))
  (Default|UpdateMoney (Variables|Default|GetPlayerUI)))

(event Custom|HealthManaRegeneration
  (bind _player (CallFunction|GetPlayer))
  (bind _playerui (Variables|Default|GetPlayerUI))
  (Utilities|FlowControl|Delay 1.0 :!label _label)
  (Utilities|FlowControl|Sequence
    (:then_0
      (if (<= (+ (Variables|/Game/Blueprint/BP_Character.BP_Character_C|GetMana _player) 1) (Variables|Default|GetManaMax))
        (bind _output_get (Variables|/Game/Blueprint/BP_Character.BP_Character_C|SetMana _player (+ (Variables|/Game/Blueprint/BP_Character.BP_Character_C|GetMana _player) 1)))
        (Utilities|IsValid _playerui
          (:Is%20Valid
            (Default|UpdateMana _playerui (Math|Conversions|ToFloat(Integer) _output_get))))
        (else
          (goto _label))))
    (:then_1
      (if (<= (+ (Variables|/Game/Blueprint/BP_Character.BP_Character_C|GetHealth _player) 1) (Variables|Default|GetHealthMax))
        (bind _output_get_2 (Variables|/Game/Blueprint/BP_Character.BP_Character_C|SetHealth _player (+ (Variables|/Game/Blueprint/BP_Character.BP_Character_C|GetHealth _player) 1)))
        (Utilities|IsValid _playerui
          (:Is%20Valid
            (Default|UpdateHealth _playerui (Math|Conversions|ToFloat(Integer) _output_get_2))))))
    (:then_2
      (goto _label))))

(event Custom|CastFireball
  (Game|SpawnActorfromClass "/Game/Blueprint/BP_Fireball.BP_Fireball_C" (Transformation|GetWorldTransform (Variables|/Game/Blueprint/BP_Player.BP_Player_C|GetSpellCastZone (CallFunction|GetPlayer))) "Undefined" "MultiplyWithRoot" 0 0))

(event Custom|ShieldPlayer
  (bind _player (CallFunction|GetPlayer))
  (bind _sphere (Variables|/Game/Blueprint/BP_Player.BP_Player_C|GetSphere _player))
  (bind _relativerotation (Variables|/Script/Engine.SceneComponent|GetRelativeRotation _sphere))
  (Variables|/Game/Blueprint/BP_Player.BP_Player_C|SetIsShielded _player true)
  (Rendering|SetVisibility _sphere true false)
  (Timeline|Timeline Play
    (:Update
      (Transformation|SetRelativeRotation _sphere (Math|Rotator|MakeRotator (.roll _relativerotation) (.pitch _relativerotation) (+ (.yaw _relativerotation) 2.0)) false false))
    (:Finished
      (Variables|/Game/Blueprint/BP_Player.BP_Player_C|SetIsShielded _player false)
      (Rendering|SetVisibility _sphere false false))))

(event Custom|CastEarthquake
  (bind _returnvalue (Game|SpawnActorfromClass "/Game/Blueprint/BP_Earthquake.BP_Earthquake_C" (Transformation|GetActorTransform (CallFunction|GetPlayer)) "Undefined" "MultiplyWithRoot" 0 0))
  (Utilities|FlowControl|Delay 0.5)
  (Actor|DestroyActor _returnvalue))

(event Input|EnhancedActionEvents|EnhancedInputActionIA_SetDestination_Click
  (params (ActionValue :type Boolean) (ElapsedSeconds :type Float%20%28double-precision%29) (TriggeredSeconds :type Float%20%28double-precision%29) (InputAction :type Input%20Action%20Object%20Reference :default "/Game/TopDown/Input/Actions/IA_SetDestination_Click.IA_SetDestination_Click"))
  (bind (_hit _location) (CallFunction|GetLocationUnderCursor))
  (bind _returnvalue (Pawn|GetControlledPawn))
  (:Triggered
    (if (not (Variables|Default|GetPlayerIsFrozen))
      (if (not (Variables|Default|GetPlayer_IsCastingSpell))
        (if _hit
          (bind _output_get (Variables|Default|SetCachedDestination _location))
          (CallFunction|Follow _output_get)
          (Transformation|SetActorRotation _returnvalue (Math|Rotator|MakeRotator 0.0 0.0 (.yaw (Math|Rotator|FindLookatRotation (Transformation|GetActorLocation _returnvalue) _output_get))))))))
  (:Started
    (AI|Navigation|StopMovement))
  (:Canceled
    (if (not (Variables|Default|GetPlayerIsFrozen)) :!label _label
      (if true
        (CallFunction|Moveto (Variables|Default|GetCachedDestination)))))
  (:Completed
    (goto _label)))

(event EventBeginPlay
  (bind _returnvalue (PlayerController|LocalPlayerSubsystems|GetEnhancedInputLocalPlayerSubsystem))
  (Utilities|FlowControl|Sequence
    (:then_0
      (Utilities|IsValid _returnvalue
        (:Is%20Valid
          (Input|AddMappingContext _returnvalue "/Game/TopDown/Input/IMC_Default.IMC_Default" 0 "(bIgnoreAllPressedKeysUntilRelease=True,bForceImmediately=False,bNotifyUserSettings=False)")
          (Variables|Default|SetbShowMouseCursor true))))
    (:then_1
      (CallFunction|SetPlayerUI)
      (CallFunction|HealthManaRegeneration)
      (Rendering|SetVisibility (Variables|/Game/Blueprint/BP_Player.BP_Player_C|GetSphere (CallFunction|GetPlayer)) false false))))

(event Input|KeyboardEvents|A
  (params (Key :type Key%20Structure :default "None"))
  (bind _player (CallFunction|GetPlayer))
  (bind _activespell (Variables|Default|GetActiveSpell))
  (bind _spellanimation (Variables|/Game/DataAsset/BP_DA_Spell.BP_DA_Spell_C|GetSpellAnimation _activespell))
  ;[0.15 0.15 0.15 0.5] Cast a spell and launch animation
  (:Pressed
    (if (not (Variables|Default|GetPlayerIsFrozen))
      (if (not (Variables|Default|GetPlayer_IsCastingSpell))
        (Variables|Default|SetPlayerIsFrozen true)
        (AI|Navigation|StopMovement)
        (bind _output_get (Variables|Default|SetPlayer_IsCastingSpell true))
        (Variables|/Game/Blueprint/BP_Player.BP_Player_C|SetIsCastingSpell _player _output_get)
        (Variables|Default|SetActiveSpellAnimation _spellanimation)
        (Utilities|FlowControl|Delay (- (Animation|GetPlayLength _spellanimation) 1.0))
        (Default|LaunchSpell _activespell _player (Variables|Default|GetPlayerUI))
        (Utilities|FlowControl|Delay 0.7)
        (bind _output_get_2 (Variables|Default|SetPlayer_IsCastingSpell false))
        (Variables|/Game/Blueprint/BP_Player.BP_Player_C|SetIsCastingSpell (CallFunction|GetPlayer) _output_get_2)
        (Variables|Default|SetPlayerIsFrozen false)))))

(event Input|MouseEvents|MouseWheelUp
  (params (Key :type Key%20Structure :default "None"))
  (bind _spelllibrary (Variables|Default|GetSpellLibrary))
  (:Pressed
    (if (== (+ (Variables|Default|GetSpellIndex) 1) (Utilities|Array|Length _spelllibrary))
      (Variables|Default|SetSpellIndex 0)
      (else
        (Variables|Default|SetSpellIndex (+ (Variables|Default|GetSpellIndex) 1))))
    (bind _output_get (Variables|Default|SetActiveSpell (Utilities|Array|Get(acopy) _spelllibrary (Variables|Default|GetSpellIndex))))
    (Default|UpdateActiveSpell (Variables|Default|GetPlayerUI) (Variables|/Game/DataAsset/BP_DA_Spell.BP_DA_Spell_C|GetName _output_get))))

(event Input|MouseEvents|MouseWheelDown
  (params (Key :type Key%20Structure :default "None"))
  (bind _spelllibrary (Variables|Default|GetSpellLibrary))
  (:Pressed
    (if (< (- (Variables|Default|GetSpellIndex) 1) 0)
      (Variables|Default|SetSpellIndex (- (Utilities|Array|Length _spelllibrary) 1))
      (else
        (Variables|Default|SetSpellIndex (- (Variables|Default|GetSpellIndex) 1))))
    (bind _output_get (Variables|Default|SetActiveSpell (Utilities|Array|Get(acopy) _spelllibrary (Variables|Default|GetSpellIndex))))
    (Default|UpdateActiveSpell (Variables|Default|GetPlayerUI) (Variables|/Game/DataAsset/BP_DA_Spell.BP_DA_Spell_C|GetName _output_get))))

(event Input|KeyboardEvents|E
  (params (Key :type Key%20Structure :default "None"))
  (bind _player (CallFunction|GetPlayer))
  (:Pressed
    (Utilities|IsValid (Variables|/Game/Blueprint/BP_Player.BP_Player_C|GetTrader _player)
      (:Is%20Valid
        (if (not (Variables|Default|GetPlayerIsFrozen))
          (Variables|Default|SetPlayerIsFrozen true)
          (Default|Buy _player))))))

(fn ConstructionScript)

(fn Moveto
  (params (location :type Vector%20%28by%20ref%29))
  (AI|Navigation|SimpleMovetoLocation self location))

(fn GetLocationUnderCursor
  (bind _hitresult (Game|Player|GetHitResultUnderCursorbyChannel "TraceTypeQuery1" true))
  (bind (_bblockinghit _binitialoverlap _time _distance _location) (Collision|BreakHitResult _hitresult))
  (return _bblockinghit _location))

(fn Follow
  (params (Location :type Vector))
  (bind _returnvalue (Pawn|GetControlledPawn))
  (Pawn|Input|AddMovementInput _returnvalue (Math|Vector|GetUnitDirection(Vector) (Transformation|GetActorLocation _returnvalue) Location) 1.0 false))

(fn GetNewSpell
  (params (NewSpell :type BP%20DA%20Spell%20Object%20Reference))
  (Utilities|Array|Add (Variables|Default|GetSpellLibrary) NewSpell))