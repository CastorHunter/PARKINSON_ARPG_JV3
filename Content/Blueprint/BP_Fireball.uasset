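; BP_Fireball is a projectile that flies forward and damages any BP_Character it overlaps.
; A Timeline started on BeginPlay drives movement, stepping the actor along its forward vector by a fixed distance per update, without sweep or delta-time scaling.
; Overlaps and the Timeline's end share one destroy path, which skips destruction when the overlap event's actor is a BP_AcidBall.
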(event EventBeginPlay
  (bind _self self)
  (Timeline|Timeline Play
    (:Update
      (Transformation|SetActorLocation _self (+ (Transformation|GetActorLocation _self) (* (Transformation|GetActorForwardVector _self) (Math|Float|MakeLiteralFloat 9.0))) false false))
    (:Finished
      (if (not (.bSuccess (Utilities|Casting|CastToBP_AcidBall (stale Collision|EventActorBeginOverlap OtherActor))))
        (Actor|DestroyActor)))))

(event Collision|EventActorBeginOverlap
  (params (OtherActor :type Actor%20Object%20Reference))
  (bind _asbp_character (Utilities|Casting|CastToBP_Character OtherActor)
    (:then
      (Default|TakeDamages _asbp_character 10))
    (:CastFailed
      _))
  (if (not (.bSuccess (Utilities|Casting|CastToBP_AcidBall OtherActor)))
    (Actor|DestroyActor)))

(fn ConstructionScript)