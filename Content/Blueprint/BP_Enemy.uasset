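; BP_Enemy is an enemy actor that takes damage, can be stunned and can turn to face the player.
; BeStunned switches the CanMove enum on its AI controller's Blackboard, then restores it after a delay.
; TakeDamages lowers Health to a floor of zero; on death it awards the player money, refreshes the money UI and destroys the enemy.
; OrientToPlayer snaps the actor's rotation toward the player's location.
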(event Custom|BeStunned
  (params (TimeBeingStunned :type Float%20%28double-precision%29))
  (bind _returnvalue (Pawn|GetController))
  (bind _returnvalue_2 (Utilities|Name|MakeLiteralName "CanMove"))
  (bind _returnvalue_3 (AI|GetBlackboard _returnvalue))
  (AI|Components|Blackboard|SetValueasEnum _returnvalue_3 _returnvalue_2 (Utilities|Enum|LiteralenumE_EnemyState "NewEnumerator1"))
  (Utilities|FlowControl|Delay TimeBeingStunned)
  (AI|Components|Blackboard|SetValueasEnum _returnvalue_3 _returnvalue_2 (Utilities|Enum|LiteralenumE_EnemyState "NewEnumerator0")))

(event EventBeginPlay
  (|CallParentFunction) ; This node is disabled and will not be called.\nDrag off pins to build functionality.
)

(event Collision|EventActorBeginOverlap
  (params (OtherActor :type Actor%20Object%20Reference))
  (|CallParentFunction OtherActor) ; This node is disabled and will not be called.\nDrag off pins to build functionality.
)

(event EventTick
  (params (DeltaSeconds :type Float%20%28single-precision%29))
  (|CallParentFunction DeltaSeconds) ; This node is disabled and will not be called.\nDrag off pins to build functionality.
)

(fn ConstructionScript
  (|CallParentFunction))

(fn OrienttoPlayer
  (Transformation|SetActorRotation (Math|Rotator|FindLookatRotation (Transformation|GetActorLocation) (Transformation|GetActorLocation (CallFunction|GetPlayer)))))

(fn TakeDamages
  (params (Damages :type Integer))
  (bind _player (CallFunction|GetPlayer))
  ;[0.15 0.15 0.15 0.5] Deduce life, with a min to 0
  (if (> (- (Variables|Default|GetHealth) Damages) 0)
    (bind _output_get (Variables|Default|SetHealth (- (Variables|Default|GetHealth) Damages)))
    (return _output_get)
    (else
      (bind _output_get_2 (Variables|Default|SetHealth 0))
      (Variables|/Game/Blueprint/BP_Player.BP_Player_C|SetMoney _player (+ (Variables|/Game/Blueprint/BP_Player.BP_Player_C|GetMoney _player) 1))
      (Default|UpdateMoney (Variables|/Game/Blueprint/BP_PlayerController.BP_PlayerController_C|GetPlayerUI (.AsBP%20Player%20Controller (Utilities|Casting|CastToBP_PlayerController (Game|GetPlayerController 0)))))
      (Actor|DestroyActor)
      (return _output_get_2))))