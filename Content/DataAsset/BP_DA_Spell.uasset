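; Spell data asset whose LaunchSpell function casts a mana-costed spell for a given caster.
; If the caster's Mana covers ManaCost, it deducts the cost and prints a launch message with the spell's name.
; It then calls Launch on each action in the Actions list of the caster controller's ActiveSpell, rather than reading its own list, passing in the BP_PlayerController.
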(fn LaunchSpell
  (params (Caster :type BP%20Character%20Object%20Reference))
  (bind _returnvalue (Pawn|GetController Caster))
  (bind _manacost (Variables|Default|GetManaCost))
  (bind _asbp_player_controller (Utilities|Casting|CastToBP_PlayerController _returnvalue))
  ;[0.15 0.15 0.15 0.5] Check if the caster has enough mana, and then deduces the necessary amount
  (if (>= (Variables|/Game/Blueprint/BP_Character.BP_Character_C|GetMana Caster) _manacost)
    (Variables|/Game/Blueprint/BP_Character.BP_Character_C|SetMana Caster (- (Variables|/Game/Blueprint/BP_Character.BP_Character_C|GetMana Caster) _manacost))
    ;[0.15 0.15 0.15 0.5] Spell is Launched
    (Development|PrintString 0 (Utilities|String|Append (Utilities|String|ToString(Name) (Variables|Default|GetName)) " is launched !"))
    (for _array_element (Variables|/Script/MyProject2.SpellDataAsset|GetActions (Variables|/Game/Blueprint/BP_PlayerController.BP_PlayerController_C|GetActiveSpell _asbp_player_controller))
      (Class|SpellAction|Launch _array_element _asbp_player_controller))))